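; Player controller that applies a chosen saved game state: music time, per-row choices and player position.
; OnGameStateChosenEvent looks up the state by index, resumes the game mode's SoundVis spectrum at that time, rebuilds GameStateStruct and broadcasts the change.
; It also moves the pawn when the saved position is non-zero.
; BeginPlay is empty; the config read, choice widget and event binding sit in disconnected nodes.
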(event `self.ReceiveBeginPlay`
  ;[1 1 1] Read Game State Variables From Configuration File
)

(event `OnGameStateChosenEvent` :!signature `self.OnGameStateChosen`
  (params (Index :type Integer))
  (bind (_musictime _playerposition _choicesperrow) (break `ChoicesPerRow` (`BlueprintMapLibrary.Map_Find` (`self.Choices`) Index)))
  ;[1 1 1] Read Game State Variables From Configuration File
  (set `self.GameStateStruct` (`self.NULL`))
  (bind _output_get (set `self.MusicTimer` _musictime))
  (`|ExecutionSequence`
    (:`then_0`
      (bind _asbp_enhanced_game_mode (cast `/Game/BP_EnhancedGameMode` (`GameplayStatics.GetGameMode`)))
      (bind _soundvis (`/Game/BP_EnhancedGameMode.SoundVis` _asbp_enhanced_game_mode))
      (`SoundVisComponent.BP_PauseCalculatingFrequencySpectrum` _soundvis)
      (`SoundVisComponent.BP_ResumeCalculatingFrequencySpectrumAtSpecificTime` _soundvis _output_get))
    (:`then_1`
      (bind _keys (`BlueprintMapLibrary.Map_Keys` _choicesperrow))
      (for _array_element _keys
        (bind (_value _returnvalue) (`BlueprintMapLibrary.Map_Find` _choicesperrow _array_element))
        (if _returnvalue
          (`KismetArrayLibrary.Array_Add` (`self.GameStateStruct`) (make `/Game/GameStateStruct` _array_element _value))))
      (`self.OnChangeGameState`))
    (:`then_2`
      (if (!= (0.0 0.0 0.0) _playerposition)
        (`self.K2_SetActorLocation` (`GameplayStatics.GetPlayerPawn` 0) _playerposition false false)))))

(fn `UserConstructionScript`)