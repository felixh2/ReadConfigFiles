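; Game mode that plays a hard-coded music file through SoundVis and lets game states be chosen from config-file data.
; BeginPlay loads the track, starts spectrum analysis, reads GameChoices and shows the choices widget.
; Choosing a state seeks the music, rebuilds GameStateStruct, broadcasts OnGameStateChanged and moves the player if a position is set.
; Tick only prints offset-corrected music time, repeating it past fixed thresholds as apparent placeholders.
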(event `self.ReceiveBeginPlay`
  (bind _soundvis (`self.SoundVis`))
  ;[1 1 1] Music
  (`KismetSystemLibrary.PrintString` "Game Mode Reporting")
  (`|ExecutionSequence`
    (:`then_1`
      (`SoundVisComponent.BP_LoadSoundFileFromHD` _soundvis "C:/Git Repositories/ReadFromConfigFile/Content/Hero.ogg")
      (add `SoundVisComponent.OnFileLoadCompleted` _soundvis (delegate `OnFileLoadCompleted_Event_0`))
      ;[1 1 1] Comment
      (add `self.OnGameStateChosen` (delegate `OnGameStateChosen_Event_0`))
      (bind _returnvalue (`self.ReadFromConfigFile1`))
      (set `self.GameChoices` _returnvalue)
      (bind _returnvalue_2 (`|CreateWidget` "/Game/BPW_GameChoicesWidget.BPW_GameChoicesWidget_C"))
      (`UserWidget.AddToViewport` _returnvalue_2 0))))

(event `OnFileLoadCompleted_Event_0`
  (params (SoundWaveRef :type "SoundWave Object Reference"))
  ;[1 1 1] Music
  (`SoundVisComponent.BP_StartCalculatingFrequencySpectrum` (`self.SoundVis`) SoundWaveRef 0.0))

(event `OnGameStateChosen_Event_0` :!signature `self.OnGameStateChosen`
  (params (Index :type Integer))
  (bind (_musictime _playerposition _choicesperrow) (break `ChoicesPerRow1` (`BlueprintMapLibrary.Map_Find` (`self.GameChoices`) Index)))
  ;[1 1 1] Comment
  (set `self.GameStateStruct` (`self.NULL`))
  (bind _output_get (set `self.SelectedMusicTime` _musictime))
  (`|ExecutionSequence`
    (:`then_0`
      (set `self.MusicTimerOffset` (`SoundVisComponent.GetCurrentPlayBackTime` (`self.SoundVis`)))
      (bind _asbp_enhanced_game_mode (cast `/Game/BP_EnhancedGameMode` (`GameplayStatics.GetGameMode`)))
      (bind _soundvis (`/Game/BP_EnhancedGameMode.SoundVis` _asbp_enhanced_game_mode))
      (`SoundVisComponent.BP_PauseCalculatingFrequencySpectrum` _soundvis)
      (`SoundVisComponent.BP_ResumeCalculatingFrequencySpectrumAtSpecificTime` _soundvis _output_get))
    (:`then_1`
      (bind _keys (`BlueprintMapLibrary.Map_Keys` _choicesperrow))
      (for _array_element _keys
        (bind (_value _returnvalue) (`BlueprintMapLibrary.Map_Find` _choicesperrow _array_element))
        (if _returnvalue
          (`KismetArrayLibrary.Array_Add` (`self.GameStateStruct`) (make `/Game/GameStateStruct` _array_element _value))))
      (`self.OnGameStateChanged`))
    (:`then_2`
      (if (!= (0.0 0.0 0.0) _playerposition)
        (`self.K2_SetActorLocation` (`GameplayStatics.GetPlayerPawn` 0) _playerposition false false)))))

(event `self.ReceiveTick`
  (params (DeltaSeconds :type "Float (single-precision)"))
  (bind _returnvalue (+ (- (`SoundVisComponent.GetCurrentPlayBackTime` (`self.SoundVis`)) (`self.MusicTimerOffset`)) (`self.SelectedMusicTime`)))
  ;[1 1 1] Comment
  (`KismetSystemLibrary.PrintString` (`KismetStringLibrary.Conv_DoubleToString` _returnvalue))
  (`|ExecutionSequence`
    (:`then_0`
      (if (> _returnvalue 20.0)
        (`KismetSystemLibrary.PrintString` (`KismetStringLibrary.Conv_DoubleToString` _returnvalue) :!label _label)))
    (:`then_1`
      (if (> _returnvalue 50.0)
        (goto _label)))
    (:`then_2`
      (if (> _returnvalue 80.0)
        (goto _label)))
    (:`then_3`
      (if (> _returnvalue 100.0)
        (goto _label)))
    (:`then_4`
      (if (> _returnvalue 120.0)
        (goto _label)))
    (:`then_5`
      (if (> _returnvalue 160.0)
        (goto _label)))
    (:`then_6`
      (if (> _returnvalue 180.0)
        (goto _label)))))

(fn `UserConstructionScript`)